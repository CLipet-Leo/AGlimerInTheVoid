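; BP_ConfirmationButton is an interactable button in Puzzle02 that acts as a puzzle condition.
; Interact calls Activate, which, like Deactivate, sets PuzzleState and broadcasts it through OnConditionStateChanged with debug prints.
; Reset restores the deactivated state without broadcasting.
; Getters expose puzzle state and interaction settings, while GetWidgetRootComp returns no component.
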(event EventReset
  (Variables|Default|SetPuzzleState "NewEnumerator0"))

(event Collision|EventActorBeginOverlap
  (params (OtherActor :type Actor%20Object%20Reference)))

(event EventTick
  (params (DeltaSeconds :type Float%20%28single-precision%29)))

(event EventInteract
  (params (InteractActorRef :type Actor%20Object%20Reference))
  (CallFunction|Activate)
  (Development|PrintString (Utilities|String|Append (Utilities|GetDisplayName InteractActorRef) " interact with " (Utilities|GetDisplayName self)) true false "(R=0.000000,G=0.200265,B=1.000000,A=1.000000)"))

(event EventBeginPlay)

(event EventActivate
  (bind _output_get (Variables|Default|SetPuzzleState "NewEnumerator2"))
  (Default|CallOnConditionStateChanged _output_get self)
  (Development|PrintString (Utilities|String|EnumtoString _output_get)))

(event EventDeactivate
  (bind _output_get (Variables|Default|SetPuzzleState "NewEnumerator0"))
  (Default|CallOnConditionStateChanged _output_get self)
  (Development|PrintString (Utilities|String|EnumtoString _output_get)))

(fn ConstructionScript)

(fn GetPuzzleState
  (return (Variables|Default|GetPuzzleState)))

(fn GetCanInteract
  (return (Variables|Interaction|GetCan%20Interact)))

(fn GetHoldDuration
  (return (Variables|Interaction|GetDuration)))

(fn GetInteractionType
  (return (Variables|Interaction|GetInteractionType)))

(fn GetWidgetRootComp
  (return 0))