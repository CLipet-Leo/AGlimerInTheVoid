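; BP_PressurePlateB is a puzzle pressure plate that is active while the third-person character overlaps its box.
; A timeline lowers the plate mesh on overlap and reverses when the overlap ends.
; Activate and Deactivate set PuzzleState and broadcast it with the plate as caller through OnConditionStateChanged.
; Reset restores the default state silently, and GetPuzzleState returns a fixed value rather than PuzzleState.
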(event OnComponentBeginOverlap(Box)
  (params (OverlappedComponent :type Primitive%20Component%20Object%20Reference) (OtherActor :type Actor%20Object%20Reference) (OtherComp :type Primitive%20Component%20Object%20Reference) (OtherBodyIndex :type Integer) (bFromSweep :type Boolean) (SweepResult :type Hit%20Result%20Structure%20%28by%20ref%29))
  (Utilities|Casting|CastToBP_ThirdPersonCharacter OtherActor)
  (Variables|Default|SetbIsActive true)
  (CallFunction|Activate)
  (bind _height (Timeline|Timeline Play)
    (:Update
      (Transformation|SetRelativeLocation (Variables|Default|GetPlate) (Math|Vector|MakeVector 0.0 0.0 (Math|Float|Lerp 21.0 8.0 _height)) false false))))

(event OnComponentEndOverlap(Box)
  (params (OverlappedComponent :type Primitive%20Component%20Object%20Reference) (OtherActor :type Actor%20Object%20Reference) (OtherComp :type Primitive%20Component%20Object%20Reference) (OtherBodyIndex :type Integer))
  (Utilities|Casting|CastToBP_ThirdPersonCharacter OtherActor)
  (Variables|Default|SetbIsActive false)
  (CallFunction|Deactivate)
  (bind _height (Timeline|Timeline Reverse)
    (:Update
      (Transformation|SetRelativeLocation (Variables|Default|GetPlate) (Math|Vector|MakeVector 0.0 0.0 (Math|Float|Lerp 21.0 8.0 _height)) false false))))

(event EventReset
  (Variables|Default|SetPuzzleState "NewEnumerator0"))

(event EventActivate
  (bind _output_get (Variables|Default|SetPuzzleState "NewEnumerator2"))
  (Default|CallOnConditionStateChanged _output_get self))

(event EventDeactivate
  (bind _output_get (Variables|Default|SetPuzzleState "NewEnumerator0"))
  (Default|CallOnConditionStateChanged _output_get self))

(fn ConstructionScript)

(fn GetPuzzleState
  (return "NewEnumerator0"))