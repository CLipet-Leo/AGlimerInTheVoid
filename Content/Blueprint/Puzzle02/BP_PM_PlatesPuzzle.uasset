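; Puzzle manager for a four-stage lever and pressure plate puzzle, with ExpectedOrder holding a lever/plate pair per stage.
; A triggered lever resets the other still-interactable condition actors.
; The correct plate with its lever completed locks that lever, fires the stage effect and advances; the last stage solves the puzzle.
; BeginPlay builds a sequence condition strategy, but the checks here use their own stage logic.
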(event EventBeginPlay
  (bind _expected_order (Variables|Sequence|GetExpected%20Order))
  (|CallParentFunction)
  (CallFunction|CheckActorsValidity (Variables|Sequence|GetExpected%20Order))
  (bind _returnvalue (Game|ConstructObjectfromClass "/Game/Blueprint/Systems/PuzzleSystem/BP_Condition_Sequence.BP_Condition_Sequence_C"))
  (bind _output_get (Variables|Sequence|SetConditionStrategy _returnvalue))
  (Variables|/Game/Blueprint/Systems/PuzzleSystem/BP_Condition_Sequence.BP_Condition_Sequence_C|SetExpectedOrder _output_get _expected_order)
  (Default|Init _output_get (Variables|Default|GetConditionActors))
  (for _array_element _expected_order
    (Development|PrintString (Utilities|GetDisplayName _array_element))))

(event EventOnStateChanged
  (params (newState :type E_PuzzleState%20Enum :default "NewEnumerator0") (callerActor :type Actor%20Object%20Reference))
  (bind _bconditionsmet (CallFunction|CheckConditions callerActor))
  (if _bconditionsmet
    (CallFunction|SolvePuzzle)))

(fn ConstructionScript
  (|CallParentFunction))

(fn CheckConditions
  (params (CallerActor :type Actor%20Object%20Reference))
  (if (Variables|Default|GetbPuzzleSolved)
    (return false)
    (else
      (bind _conditions_met (CallFunction|CheckPuzzleStep CallerActor))
      (return _conditions_met))))

(fn CheckPuzzleStep
  (params (TriggeredActor :type Actor%20Object%20Reference))
  (bind _conditionactors (Variables|Default|GetConditionActors))
  (Utilities|FlowControl|Sequence
    (:then_0
      (Utilities|Casting|CastToBP_Lever TriggeredActor)
      (for (_array_element _array_index) _conditionactors
        (bind _currentlevelindex (CallFunction|FindCurrentLever _conditionactors TriggeredActor))
        (bind _caninteract (Class|BPIInteractable|GetCanInteract(Message) _array_element))
        (if _caninteract
          (if (not (== _currentlevelindex _array_index))
            (Default|Reset _array_element)))))
    (:then_1
      (if (>= (Variables|Default|GetCurrentStage) 4)
        (return false)
        (else
          (bind _bispressureplate (CallFunction|CheckifPressurePlate TriggeredActor))
          (if _bispressureplate
            (bind _asbp_lever (Utilities|Casting|CastToBP_Lever (Utilities|Array|Get(acopy) (Variables|Sequence|GetExpected%20Order) (* (Variables|Default|GetCurrentStage) 2))))
            (bind _state (Default|GetPuzzleState _asbp_lever))
            (switch Utilities|FlowControl|Switch|SwitchonE_PuzzleState _state
              (:NewEnumerator2
                (if (== (Utilities|Array|Get(acopy) (Variables|Sequence|GetExpected%20Order) (+ (* (Variables|Default|GetCurrentStage) 2) 1)) TriggeredActor)
                  (Development|PrintString (Utilities|String|Append "You Completed Stage : " (Utilities|String|ToString(Integer) (+ (Variables|Default|GetCurrentStage) 1))))
                  (Default|SetCanInteract _asbp_lever false)
                  (Default|CallEffect (Utilities|Array|Get(acopy) (Variables|Default|GetEffectActors) (Variables|Default|GetCurrentStage)))
                  (bind _output_get (Variables|Default|SetCurrentStage (+ (Variables|Default|GetCurrentStage) 1)))
                  (if (>= _output_get 4)
                    (return true)))))
            (else
              (return false))))))))

(fn CheckifPressurePlate
  (params (Object :type Actor%20Object%20Reference))
  (Utilities|Casting|CastToBP_PressurePlateA Object
    (:then
      (return true))
    (:CastFailed
      (Utilities|Casting|CastToBP_PressurePlateB Object
        (:then
          (return true))
        (:CastFailed
          (Utilities|Casting|CastToBP_PressurePlateD Object
            (:then
              (return true))
            (:CastFailed
              (Utilities|Casting|CastToBP_PressurePlateC Object
                (:then
                  (return true))
                (:CastFailed
                  (return false))))))))))

(fn CheckforActivatedLevers
  (params (Actors :type Array%20of%20Actor%20Object%20References))
  (Development|PrintString "Checking Levers")
  (for _array_element Actors
    (bind _asbp_lever (Utilities|Casting|CastToBP_Lever _array_element))
    (bind _state (Default|GetPuzzleState _asbp_lever))
    (switch Utilities|FlowControl|Switch|SwitchonE_PuzzleState _state
      (:NewEnumerator2
        (bind _output_get (Variables|Default|SetActivatedLevers (+ (Variables|Default|GetActivatedLevers) 1)))
        (Development|PrintString (Utilities|String|ToString(Integer) _output_get))
        (if (>= _output_get 2)
          (return true)
          (else
            (return false)))))))

(fn ResetAllLevers
  (params (Actors :type Array%20of%20Actor%20Object%20References))
  (Development|PrintString "Reseting Levers")
  (for _array_element Actors
    (bind _asbp_lever (Utilities|Casting|CastToBP_Lever _array_element))
    (Variables|Default|SetActivatedLevers 1)
    (Default|Reset _asbp_lever)))

(fn FindCurrentLever
  (params (AllActors :type Array%20of%20Actor%20Object%20References) (Actor :type Actor%20Object%20Reference))
  (for (_array_element _array_index) AllActors
    (if (== _array_element Actor)
      (bind _output_get (Variables|Default|SetCurrentLeverIndex _array_index))
      (return _output_get))))