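; BP_Lever is an interactable puzzle lever that toggles on and off, swinging its Sphere component via a timeline.
; Each interaction messages receiver actors implementing BPI_Receiver, sets the puzzle state and broadcasts the condition change.
; Reset restores the puzzle state and reverses the animation, but leaves IsActive untouched and notifies nothing.
; Getters expose puzzle state and interaction settings.
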(event EventReset
  (Variables|Default|SetPuzzleState "NewEnumerator0")
  (bind _rotation (Timeline|Timeline Reverse)
    (:Update
      (Transformation|SetRelativeRotation (Variables|Default|GetSphere) (Math|Rotator|MakeRotator (Math|Float|Lerp -4e+01 4e+01 _rotation) 0.0 0.0) false false))))

(event EventSetCanInteract
  (params (newCanInteract :type Boolean))
  (Variables|Default|SetCanInteract newCanInteract))

(event EventInteract
  (params (InteractActorRef :type Actor%20Object%20Reference))
  (bind _output_get (Variables|Default|SetbIsActive (not (Variables|Default|GetbIsActive))))
  (CallFunction|EmittMessage)
  (if _output_get
    (CallFunction|Activate)
    (bind _rotation (Timeline|Timeline Play)
      (:Update
        (Transformation|SetRelativeRotation (Variables|Default|GetSphere) (Math|Rotator|MakeRotator (Math|Float|Lerp -4e+01 4e+01 _rotation) 0.0 0.0) false false)))
    (else
      (CallFunction|Deactivate)
      (Timeline|Timeline Reverse))))

(event EventActivate
  (bind _output_get (Variables|Default|SetPuzzleState "NewEnumerator2"))
  (Default|CallOnConditionStateChanged _output_get self))

(event EventDeactivate
  (bind _output_get (Variables|Default|SetPuzzleState "NewEnumerator0"))
  (Default|CallOnConditionStateChanged _output_get self))

(fn ConstructionScript)

(fn EmittMessage
  (for _array_element (Variables|Default|GetReceiverActors)
    (if (Utilities|DoesObjectImplementInterface _array_element "/Game/Blueprint/Systems/InteractionSystem/BPI_Receiver.BPI_Receiver_C")
      (Class|BPIReceiver|ReceiveMessage(Message) _array_element (Variables|Default|GetbIsActive) self))))

(fn GetPuzzleState
  (return (Variables|Default|GetPuzzleState)))

(fn GetCanInteract
  (return (Variables|Default|GetCanInteract)))

(fn GetHoldDuration
  (return (Variables|Default|GetDuration)))

(fn GetInteractionType
  (return (Variables|Default|GetType)))

(fn GetWidgetRootComp
  (return 0))