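; Blueprint function library with shared helpers for UI access, character classification and audio volume.
; GetUIManager returns the game instance cast to UMS_UIManager.
; CastToAI reports whether an object is a Character and whether an AIController drives it.
; ChangeVolume overrides a given sound class's volume in the SCM_Master sound mix, with zero pitch and no fade, then pushes that mix.
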(fn GetUIManager
  (bind _asums_uimanager (Utilities|Casting|CastToUMS_UIManager (Game|GetGameInstance (LocalVariables|Get__WorldContext))))
  (return _asums_uimanager))

(fn CasttoAI
  (params (Object :type Actor%20Object%20Reference))
  (bind _ascharacter (Utilities|Casting|CastToCharacter Object) ; Verify if the hit is a character
    (:then
      (Utilities|Casting|CastToAIController (Pawn|GetController _ascharacter) ; If its an other ai DONT apply damage
        (:then
          (return true true))
        (:CastFailed
          (return true false))))
    (:CastFailed
      (return false false))))

(fn ChangeVolume
  (params (InSoundClass :type Sound%20Class%20Object%20Reference) (Volume :type Float%20%28single-precision%29))
  (Audio|SetSoundMixClassOverride 0 "/Game/Audio/SCM_Master.SCM_Master" InSoundClass Volume 0.0 0.0 true)
  (Audio|PushSoundMixModifier 0 "/Game/Audio/SCM_Master.SCM_Master"))