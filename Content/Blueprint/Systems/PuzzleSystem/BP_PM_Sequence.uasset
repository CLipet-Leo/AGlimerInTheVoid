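; BP_PM_Sequence is a puzzle manager that solves its puzzle based on an expected order of actors.
; On BeginPlay it validates ExpectedOrder and passes it to a newly constructed BP_Condition_Sequence, stored as its condition strategy.
; Each state change hands the calling actor to that strategy and calls SolvePuzzle when the check passes.
; Checks return false without consulting the strategy while SequenceRunning is set.
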(event EventBeginPlay
  (|CallParentFunction)
  (CallFunction|CheckActorsValidity (Variables|Sequence|GetExpected%20Order))
  (bind _returnvalue (Game|ConstructObjectfromClass "/Game/Blueprint/Systems/PuzzleSystem/BP_Condition_Sequence.BP_Condition_Sequence_C"))
  (bind _output_get (Variables|Sequence|SetConditionStrategy _returnvalue))
  (Variables|/Game/Blueprint/Systems/PuzzleSystem/BP_Condition_Sequence.BP_Condition_Sequence_C|SetExpectedOrder _output_get (Variables|Sequence|GetExpected%20Order)))

(event EventOnStateChanged
  (params (newState :type E_PuzzleState%20Enum :default "NewEnumerator0") (callerActor :type Actor%20Object%20Reference))
  (bind _bconditionsmet (CallFunction|CheckConditions callerActor))
  (if _bconditionsmet
    (CallFunction|SolvePuzzle)))

(fn ConstructionScript
  (|CallParentFunction))

(fn CheckConditions
  (params (CallerActor :type Actor%20Object%20Reference))
  (if (Variables|Sequence|GetbSequenceRunning)
    (return false)
    (else
      (bind _bconditionsmet (Default|CheckConditions (Variables|Sequence|GetConditionStrategy) CallerActor))
      (return _bconditionsmet))))