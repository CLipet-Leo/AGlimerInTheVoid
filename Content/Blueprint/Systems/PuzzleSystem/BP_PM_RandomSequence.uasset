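; Puzzle manager for a memory puzzle that flashes a random order of condition actors, then checks state changes against it.
; Reset shuffles the actors, stores three as the expected order in a BP_Condition_Sequence strategy and prints their names.
; Chained timers show and hide each step's message.
; State changes are ignored during playback or once solved; otherwise the strategy decides when the puzzle is solved.
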(event Custom|ShowNextStep
  (bind _conditionstrategy (Variables|Sequence|GetConditionStrategy))
  (bind _expectedorder (Variables|/Game/Blueprint/Systems/PuzzleSystem/BP_Condition_Sequence.BP_Condition_Sequence_C|GetExpectedOrder _conditionstrategy))
  (if (>= (Variables|Sequence|GetShowIndex) (Utilities|Array|Length _expectedorder))
    (Variables|Sequence|SetbSequenceRunning false)
    (else
      (bind _output_get (Variables|Sequence|SetCurrentShowActor (Utilities|Array|Get(acopy) _expectedorder (Variables|Sequence|GetShowIndex))))
      (Class|BPISequenceEffect|Show(Message) _output_get)
      (Utilities|Time|SetTimerbyEvent (delegate Custom|DeactivateCurrent) (* (Variables|Sequence|GetStepDuration) 0.7))
      (Math|Integer|IncrementInt (Variables|Sequence|GetShowIndex)
        (:%20%20
          (Utilities|Time|SetTimerbyEvent (EventDispatchers|CreateEvent :!event Custom|ShowNextStep) (Variables|Sequence|GetStepDuration)))))))

(event Custom|DeactivateCurrent
  (Class|BPISequenceEffect|Hide(Message) (Variables|Sequence|GetCurrentShowActor)))

(event EventBeginPlay
  (|CallParentFunction)
  (bind _returnvalue (Game|ConstructObjectfromClass "/Game/Blueprint/Systems/PuzzleSystem/BP_Condition_Sequence.BP_Condition_Sequence_C"))
  (bind _output_get (Variables|Sequence|SetConditionStrategy _returnvalue))
  (Default|Init _output_get (Variables|Default|GetConditionActors))
  (Sequence|Reset)
  (Sequence|ShowSequence))

(event EventOnStateChanged
  (params (newState :type E_PuzzleState%20Enum :default "NewEnumerator0") (callerActor :type Actor%20Object%20Reference))
  (bind _bconditionsmet (CallFunction|CheckConditions callerActor))
  (if _bconditionsmet
    (CallFunction|SolvePuzzle)))

(fn ConstructionScript
  (|CallParentFunction))

(fn CheckConditions
  (params (CallerActor :type Actor%20Object%20Reference))
  (if (or (Variables|Sequence|GetbSequenceRunning) (Variables|Default|GetbPuzzleSolved))
    (return false)
    (else
      (bind _bconditionsmet (Default|CheckConditions (Variables|Sequence|GetConditionStrategy) CallerActor))
      (return _bconditionsmet))))

(fn GenerateRandomSequence
  (params (Count :type Integer))
  (LocalVariables|SetSafeCount (Math|Integer|Clamp(Integer) Count 1 (Utilities|Array|Length (Variables|Default|GetConditionActors))))
  (bind _output_get (LocalVariables|SetShufflePool (Variables|Default|GetConditionActors)))
  (Utilities|Array|Shuffle _output_get)
  (for _index (range 1 (Utilities|LengthMinus _output_get 1))
    (bind _output_get_2 (LocalVariables|SetiCurrentIndex (- (Utilities|LengthMinus (LocalVariables|GetShufflePool) 1) _index)))
    ;[0.15 0.15 0.15 0.5] Comment
    (LocalVariables|SetjRandomIndex (Math|Random|RandomIntegerinRange 0 _output_get_2))
    (LocalVariables|SetTemp (Utilities|Array|Get(acopy) (LocalVariables|GetShufflePool) (LocalVariables|GetiCurrentIndex)))
    (Utilities|Array|SetArrayElem (LocalVariables|GetShufflePool) (LocalVariables|GetiCurrentIndex) (Utilities|Array|Get(acopy) (LocalVariables|GetShufflePool) (LocalVariables|GetjRandomIndex)))
    (Utilities|Array|SetArrayElem (LocalVariables|GetShufflePool) (LocalVariables|GetjRandomIndex) (LocalVariables|GetTemp)))
  ;[0.15 0.15 0.15 0.5] Comment
  (for _index_2 (range 0 (- (LocalVariables|GetSafeCount) 1))
    (Utilities|Array|AddUnique (LocalVariables|GetNewExpectedOrder) (Utilities|Array|Get(acopy) (LocalVariables|GetShufflePool) _index_2)))
  (return (LocalVariables|GetNewExpectedOrder)))

(fn Reset
  (bind _conditionstrategy (Variables|Sequence|GetConditionStrategy))
  (bind _newexpectedorder (Sequence|GenerateRandomSequence 3))
  (Variables|/Game/Blueprint/Systems/PuzzleSystem/BP_Condition_Sequence.BP_Condition_Sequence_C|SetExpectedOrder _conditionstrategy _newexpectedorder)
  (Default|Reset _conditionstrategy)
  (for _array_element _newexpectedorder
    (Development|PrintString (Utilities|GetDisplayName _array_element) true true "(R=0.000000,G=0.660000,B=1.000000,A=1.000000)" 4.0)))

(fn ShowSequence
  (Utilities|Time|ClearandInvalidateTimerbyHandle (Variables|Sequence|GetSequenceTimerHandle))
  (Variables|Sequence|SetShowIndex 0)
  (Variables|Sequence|SetbSequenceRunning true)
  (for _array_element (Variables|Default|GetConditionActors)
    (Class|BPIPuzzleable|Reset(Message) _array_element))
  (bind _returnvalue (Utilities|Time|SetTimerbyEvent (EventDispatchers|CreateEvent :!event Custom|ShowNextStep) (Variables|Sequence|GetStepDuration)))
  (Variables|Sequence|SetSequenceTimerHandle _returnvalue))