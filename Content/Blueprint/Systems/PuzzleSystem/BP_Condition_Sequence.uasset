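; Puzzle system condition that is met when actors trigger it in a predefined order.
; CheckConditions compares each calling actor to the ExpectedOrder entry at CurrentIndex, advancing on a match and returning true once the sequence is complete.
; A wrong actor calls Reset, which zeroes the index and calls CallOnReset, while an empty order always fails.
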(fn CheckConditions
  (params (CallerActor :type Actor%20Object%20Reference))
  (if (Utilities|Array|IsEmpty (Variables|Conditions|GetExpectedOrder))
    (return false)
    (elif (== CallerActor (Utilities|Array|Get(acopy) (Variables|Conditions|GetExpectedOrder) (Variables|Conditions|GetCurrentIndex)))
      (bind _result (Math|Integer|IncrementInt (Variables|Conditions|GetCurrentIndex))
        (:%20%20
          (if (>= _result (Utilities|Array|Length (Variables|Conditions|GetExpectedOrder)))
            (return true))))
      (else
        (CallFunction|Reset)
        (return false)))))

(fn Reset
  (Variables|Conditions|SetCurrentIndex 0)
  (Default|CallOnReset))