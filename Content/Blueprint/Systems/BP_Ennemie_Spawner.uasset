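; Enemy spawner actor that keeps one AI character of a configured class in play, respawning it after it is destroyed.
; On BeginPlay it spawns the character at its own transform, or raises a script error if no class is set.
; Each spawn creates the default controller and starts logic on that controller's StateTreeAIComponent.
; The character's OnDestroyed event clears the reference and triggers the next spawn after a configurable delay.
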(event Custom|OnSpawnNewAI
  (bind _spawnedcharacter (CallFunction|SpawnNewActor))
  (Game|AssignOnDestroyed _spawnedcharacter (delegate Custom|OnCharacterDestroyed)))

(event Custom|OnCharacterDestroyed
  (params (DestroyedActor :type Actor%20Object%20Reference))
  ;[0.15 0.15 0.15 0.5] When character is destroyed, set a delay and spawn a new ennemy after that
  (Variables|EnnemieSpawner|SetCharacterRef 0)
  (Utilities|FlowControl|Delay (Variables|Default|GetSpawnDelay))
  (CallFunction|OnSpawnNewAI))

(event EventBeginPlay
  (if (Utilities|IsValidClass (Variables|EnnemieSpawner|GetCharacterClass))
    (CallFunction|OnSpawnNewAI)
    (else
      (Utilities|Debugging|RaiseScriptError (Utilities|String|Append "Character Class for " (Utilities|GetDisplayName self) " is not well defined")))))

(fn ConstructionScript)

(fn SpawnNewActor
  (bind _returnvalue (Transformation|GetActorTransform))
  (bind (_location _rotation) (Math|Transform|BreakTransform _returnvalue))
  (bind _returnvalue_2 (Game|SpawnActorfromClass (Variables|EnnemieSpawner|GetCharacterClass) (Math|Transform|MakeTransform _location _rotation "1.000000,1.000000,1.000000") "Undefined" "MultiplyWithRoot" 0 0))
  (Pawn|SpawnDefaultController _returnvalue_2)
  (Variables|EnnemieSpawner|SetCharacterRef _returnvalue_2)
  (Development|PrintString "Spawning Ennemy" true true "(R=1.000000,G=0.000000,B=0.056656,A=1.000000)")
  ;[0.15 0.15 0.15 0.5] Start state tree logic
  (Utilities|IsValid (Actor|GetComponentbyClass (Pawn|GetController (Variables|EnnemieSpawner|GetCharacterRef)) "/Script/GameplayStateTreeModule.StateTreeAIComponent")
    (:Is%20Valid
      (AI|Logic|StartLogic (Actor|GetComponentbyClass (Pawn|GetController (Variables|EnnemieSpawner|GetCharacterRef)) "/Script/GameplayStateTreeModule.StateTreeAIComponent"))
      (return (Variables|EnnemieSpawner|GetCharacterRef)))))