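; Actor component that tracks an owner's health and death state.
; On BeginPlay it fills health to the maximum, binds to the owner's OnTakeAnyDamage and broadcasts an initialized event.
; Each hit subtracts damage clamped between zero and max, broadcasts the change with the previous value, and at zero sets IsDead and fires a depleted event.
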(event Custom|TakeDamage
  (params (DamagedActor :type Actor%20Object%20Reference) (Damage :type Float%20%28single-precision%29) (DamageType :type Damage%20Type%20Object%20Reference) (InstigatedBy :type Controller%20Object%20Reference) (DamageCauser :type Actor%20Object%20Reference))
  (bind _output_get (Variables|Default|SetPreviousHealth (Variables|Default|GetCurrentHealth)))
  (bind _output_get_2 (Variables|Default|SetCurrentHealth (Math|Float|Clamp(Float) (- (Variables|Default|GetCurrentHealth) Damage) 0.0 (Variables|Default|GetMaxHealth))))
  (Default|CallOnHealthChanged _output_get_2 _output_get)
  (if (<= (Variables|Default|GetCurrentHealth) 0.0)
    (Variables|Default|SetIsDead true)
    (Default|CallOnHealthDepleted)))

(event EventBeginPlay
  ;[0.15 0.15 0.15 0.5] Initialize health with max value and bind event to OnTakeAnyDamage
  (Variables|Default|SetCurrentHealth (Variables|Default|GetMaxHealth))
  (EventDispatchers|BindEventtoOnTakeAnyDamage (Components|GetOwner) (delegate Custom|TakeDamage))
  (Default|CallOnHealthInitialized (Variables|Default|GetMaxHealth) (Variables|Default|GetCurrentHealth)))