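; BP_CenterCrystal is an interactable crystal in the light system that lets the player set the room's color.
; On Interact, it binds ChangeColor to the player's color-changed dispatcher and calls ChangeRoomColor with the selected color at zero energy cost.
; ChangeColor switches on the player's selected color name, tinting the sphere's dynamic material instance and five point lights to match.
; It reports a short hold duration for interaction.
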(event Custom|ChangeColor
  (bind _pointlight1 (Variables|Default|GetPointLight1))
  (bind _dmi (Variables|Default|GetDMI))
  (switch string (Variables|/Game/Blueprint/ThirdPerson/BP_PlayerCharacter.BP_PlayerCharacter_C|GetSelectedColorName (Variables|Default|GetAs%20BP%20Player%20Character))
    (:Red
      (Rendering|Material|SetVectorParameterValue _dmi "Color" "(R=0.982292,G=0.000000,B=0.000000,A=1.000000)" :!class /Script/Engine.MaterialInstanceDynamic)
      (Rendering|Components|Light|SetLightColor (Variables|Default|GetPointLight) "(R=1.000000,G=0.000000,B=0.000000,A=1.000000)" true))
    (:Blue
      (Rendering|Material|SetVectorParameterValue _dmi "Color" "(R=0.000000,G=0.000000,B=1.000000,A=1.000000)" :!class /Script/Engine.MaterialInstanceDynamic)
      (Rendering|Components|Light|SetLightColor _pointlight1 "(R=0.000000,G=0.000000,B=1.000000,A=1.000000)" true))
    (:Green
      (Rendering|Material|SetVectorParameterValue _dmi "Color" "(R=0.000000,G=1.000000,B=0.000000,A=1.000000)" :!class /Script/Engine.MaterialInstanceDynamic)
      (Rendering|Components|Light|SetLightColor _pointlight1 "(R=0.000000,G=1.000000,B=0.000000,A=1.000000)" true))
    (:Purple
      (Rendering|Material|SetVectorParameterValue _dmi "Color" "(R=0.434154,G=0.000000,B=1.000000,A=1.000000)" :!class /Script/Engine.MaterialInstanceDynamic)
      (Rendering|Components|Light|SetLightColor _pointlight1 "(R=0.434154,G=0.000000,B=1.000000,A=1.000000)" true))
    (:Gold
      (Rendering|Material|SetVectorParameterValue _dmi "Color" "(R=1.000000,G=0.552012,B=0.001821,A=1.000000)" :!class /Script/Engine.MaterialInstanceDynamic)
      (Rendering|Components|Light|SetLightColor _pointlight1 "(R=1.000000,G=0.552012,B=0.001821,A=1.000000)" true))))

(event EventBeginPlay
  (bind _returnvalue (Rendering|Material|CreateDynamicMaterialInstance (Variables|Default|GetSphere) 0 "/Game/Blueprint/Systems/LightSystem/Materials/M_Crystal_Inst.M_Crystal_Inst" "None" :!class /Script/Engine.PrimitiveComponent))
  (bind _output_get (Variables|Default|SetDMI _returnvalue))
  (Rendering|Material|SetMaterial (Variables|Default|GetSphere) 0 _output_get))

(event Collision|EventActorBeginOverlap
  (params (OtherActor :type Actor%20Object%20Reference)))

(event EventTick
  (params (DeltaSeconds :type Float%20%28single-precision%29)))

(event EventInteract
  (params (InteractActorRef :type Actor%20Object%20Reference))
  (bind _asbp_player_character (Utilities|Casting|CastToBP_PlayerCharacter InteractActorRef))
  (bind _output_get (Variables|Default|SetAs%20BP%20Player%20Character _asbp_player_character))
  (EventDispatchers|BindEventtoOnColorChangedDispatcher _output_get (delegate Custom|ChangeColor))
  (Default|ChangeRoomColor _output_get (Variables|/Game/Blueprint/ThirdPerson/BP_PlayerCharacter.BP_PlayerCharacter_C|GetSelectedColor (Variables|Default|GetAs%20BP%20Player%20Character)) 0.0))

(fn ConstructionScript)

(fn GetHoldDuration
  (return 0.5))

(fn GetInteractionType
  (return "NewEnumerator1"))