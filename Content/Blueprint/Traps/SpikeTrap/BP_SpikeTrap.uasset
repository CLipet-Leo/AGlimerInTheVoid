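; Spike trap Blueprint that reacts to the third-person character entering or leaving its collider.
; On overlap begin it activates the trap with its damage amount and the character, with a flag and short delay blocking rapid re-triggering.
; On overlap end it deactivates the trap.
; Activate, deactivate and apply-damage functions only forward to the parent class, which holds the actual trap behavior.
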(event OnComponentBeginOverlap(Collider)
  (params (OverlappedComponent :type Primitive%20Component%20Object%20Reference) (OtherActor :type Actor%20Object%20Reference) (OtherComp :type Primitive%20Component%20Object%20Reference) (OtherBodyIndex :type Integer) (bFromSweep :type Boolean) (SweepResult :type Hit%20Result%20Structure%20%28by%20ref%29))
  (bind _asbp_third_person_character (Utilities|Casting|CastToBP_ThirdPersonCharacter OtherActor))
  (if (Variables|Default|GetCanActivate)
    (Variables|Default|SetCanActivate false)
    (CallFunction|ActivateTrap (Variables|Default|GetDamageAmount) _asbp_third_person_character)
    (Utilities|FlowControl|Delay 0.2)
    (Variables|Default|SetCanActivate true)))

(event OnComponentEndOverlap(Collider)
  (params (OverlappedComponent :type Primitive%20Component%20Object%20Reference) (OtherActor :type Actor%20Object%20Reference) (OtherComp :type Primitive%20Component%20Object%20Reference) (OtherBodyIndex :type Integer))
  (Utilities|Casting|CastToBP_ThirdPersonCharacter OtherActor)
  (CallFunction|DesactivateTrap))

(fn ConstructionScript)

(fn ActivateTrap
  (params (Damage :type Float%20%28double-precision%29) (Character :type BP%20Third%20Person%20Character%20Object%20Reference))
  (|CallParentFunction Damage Character))

(fn DesactivateTrap
  (|CallParentFunction))

(fn ApplyDamage
  (params (Damage :type Float%20%28double-precision%29) (Character :type BP%20Third%20Person%20Character%20Object%20Reference))
  (|CallParentFunction Damage Character))