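; Swinging axe trap that damages and knocks back the third-person character on overlap.
; A Timeline started at BeginPlay drives the pitch of RotationAxe.
; Box overlap calls ActivateTrap with the damage amount, then PushBack applies an upward impulse and one opposite the character mesh's forward vector.
; A CanActivate gate with a short delay limits retriggering, and end overlap calls DesactivateTrap.
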(event OnComponentBeginOverlap(Box)
  (params (OverlappedComponent :type Primitive%20Component%20Object%20Reference) (OtherActor :type Actor%20Object%20Reference) (OtherComp :type Primitive%20Component%20Object%20Reference) (OtherBodyIndex :type Integer) (bFromSweep :type Boolean) (SweepResult :type Hit%20Result%20Structure%20%28by%20ref%29))
  (bind _asbp_third_person_character (Utilities|Casting|CastToBP_ThirdPersonCharacter OtherActor))
  (if (Variables|Default|GetCanActivate)
    (Variables|Default|SetCanActivate false)
    (CallFunction|ActivateTrap (Variables|Default|GetDamageAmount) _asbp_third_person_character)
    (CallFunction|PushBack _asbp_third_person_character)
    (Utilities|FlowControl|Delay 0.2)
    (Variables|Default|SetCanActivate true)))

(event OnComponentEndOverlap(Box)
  (params (OverlappedComponent :type Primitive%20Component%20Object%20Reference) (OtherActor :type Actor%20Object%20Reference) (OtherComp :type Primitive%20Component%20Object%20Reference) (OtherBodyIndex :type Integer))
  (Utilities|Casting|CastToBP_ThirdPersonCharacter OtherActor)
  (CallFunction|DesactivateTrap))

(event EventBeginPlay
  (bind _newtrack_0 (Timeline|Timeline Play)
    (:Update
      (Transformation|SetRelativeRotation (Variables|Default|GetRotationAxe) (Math|Rotator|MakeRotator 0.0 _newtrack_0 0.0) false false))))

(fn ConstructionScript)

(fn PushBack
  (params (Character :type BP%20Third%20Person%20Character%20Object%20Reference))
  (bind _charactermovement (Variables|/Script/Engine.Character|GetCharacterMovement Character))
  (Physics|AddImpulse _charactermovement (* (Transformation|GetActorUpVector) "0.000000,0.000000,150.000000") true)
  (Physics|AddImpulse _charactermovement (* (Math|Vector|GetForwardVector (Variables|/Script/Engine.Character|GetMesh Character)) (* (Variables|Default|GetPushForce) -1.0)) true))