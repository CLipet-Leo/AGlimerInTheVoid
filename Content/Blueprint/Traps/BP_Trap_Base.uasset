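; Base Blueprint for traps, providing shared activation, damage and sound functions.
; Activate Trap sets the active flag, deals the passed damage to the given character and plays the SFX as a non-spatial 2D sound.
; Desactivate Trap clears the flag, and a getter exposes it.
; The event graph and construction script are empty, so activation must be triggered from outside these graphs.
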(event EventBeginPlay)

(event Collision|EventActorBeginOverlap
  (params (OtherActor :type Actor%20Object%20Reference)))

(event EventTick
  (params (DeltaSeconds :type Float%20%28single-precision%29)))

(fn ConstructionScript)

(fn ActivateTrap
  (params (Damage :type Float%20%28double-precision%29) (Character :type BP%20Third%20Person%20Character%20Object%20Reference))
  (Variables|Trap|SetbIsActive true)
  (Trap|ApplyDamage Damage Character)
  (Trap|PlaySound))

(fn DesactivateTrap
  (Variables|Trap|SetbIsActive false))

(fn ApplyDamage
  (params (Damage :type Float%20%28double-precision%29) (Character :type BP%20Third%20Person%20Character%20Object%20Reference))
  (Game|Damage|ApplyDamage Character Damage 0 0))

(fn PlaySound
  (Audio|PlaySound2D (Variables|Trap|GetSFX) 1.0 1.0 0.0 0 0))

(fn GetBisActive
  (return (Variables|Trap|GetbIsActive)))