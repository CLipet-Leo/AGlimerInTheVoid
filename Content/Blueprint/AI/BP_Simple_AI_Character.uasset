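; BP_Simple_AI_Character is a simple AI character that damages non-AI characters on contact and destroys itself.
; On possession it stores its starting location and prints a debug message naming itself and its new controller.
; On hit it ignores non-characters and characters driven by an AIController.
; For any other character it applies its configured damage and damage type, then destroys its own actor.
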(event EventPossessed
  (params (NewController :type Controller%20Object%20Reference))
  (Variables|StateTreeContext|SetStartingLocation (Transformation|GetActorLocation))
  (Development|PrintString (Utilities|String|Append (Utilities|GetDisplayName self) " : possessed by => " (Utilities|GetDisplayName NewController)) true true "(R=0.000000,G=0.067201,B=1.000000,A=1.000000)" 4.0))

(event Collision|EventHit
  (params (MyComp :type Primitive%20Component%20Object%20Reference) (Other :type Actor%20Object%20Reference) (OtherComp :type Primitive%20Component%20Object%20Reference) (bSelfMoved :type Boolean) (HitLocation :type Vector :default "0, 0, 0") (HitNormal :type Vector :default "0, 0, 0") (NormalImpulse :type Vector :default "0, 0, 0") (Hit :type Hit%20Result%20Structure%20%28by%20ref%29))
  (bind _ascharacter (Utilities|Casting|CastToCharacter Other)) ; Verify if the hit is a character
  (Utilities|Casting|CastToAIController (Pawn|GetController _ascharacter) ; If its an other ai DONT apply damage
    (:CastFailed
      (Game|Damage|ApplyDamage _ascharacter (Variables|Ennemy|GetDamage) 0 0 "/Script/Engine.DamageType")
      (Actor|DestroyActor))))

(fn ConstructionScript)