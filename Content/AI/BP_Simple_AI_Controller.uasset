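; Simple AI controller that reacts to perception updates by tracking a target and signaling its State Tree.
; When a stimulus is sensed, it stores the actor as TargetActor and sends an Attacking event tag to the StateTreeAI component.
; When sensing is lost, it saves the current target's position as LastLocation and clears the target.
; The perception-forgotten handler is an unused test stub.
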(event OnTargetPerceptionUpdated(AIPerception)
  (params (Actor :type Actor%20Object%20Reference) (Stimulus :type AI%20Stimulus%20Structure))
  (if (.bSuccessfullySensed (Utilities|Struct|BreakAIStimulus Stimulus))
    ;[0.15 0.15 0.15 0.5] If a target is sensed, call the Attacking Event
    (Variables|Default|SetTargetActor Actor)
    (Gameplay|StateTree|SendStateTreeEvent (Variables|Default|GetStateTreeAI) (Utilities|Struct|MakeStateTreeEvent "(TagName=\"AI.Event.Attacking\")") :!class /Script/GameplayStateTreeModule.StateTreeComponent)
    (else
      ;[0.15 0.15 0.15 0.5] If the target is lost, set the target to NONE
      (Variables|Default|SetLastLocation (Transformation|GetActorLocation (Variables|Default|GetTargetActor)))
      (Variables|Default|SetTargetActor 0))))

(event OnTargetPerceptionForgotten(AIPerception)
  (params (Actor :type Actor%20Object%20Reference))
  ;[0.15 0.01078 0.01078 0.5] NOT USED (tests)
)

(fn ConstructionScript)