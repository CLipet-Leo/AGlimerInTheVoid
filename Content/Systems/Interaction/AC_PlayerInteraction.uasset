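; Player interaction component that lets its owning Character use the nearest actor implementing BPI_Interactable.
; On BeginPlay it adds a range sphere whose overlaps maintain the list of interactables in reach.
; IA_Interact picks the closest one and checks its interaction type: Press fires immediately, Hold binds to a dispatcher fed by the input's elapsed time.
; Holds fire past a hardcoded threshold, and bindings clear when input completes or cancels.
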(event Custom|HandleRangeBeginOverlap
  (params (OverlappedComponent :type Primitive%20Component%20Object%20Reference) (OtherActor :type Actor%20Object%20Reference) (OtherComp :type Primitive%20Component%20Object%20Reference) (OtherBodyIndex :type Integer) (bFromSweep :type Boolean) (SweepResult :type Hit%20Result%20Structure%20%28by%20ref%29))
  ;[0.15 0.15 0.15 0.5] Add to "InteractablesInRange" if an interactable actor is in range
  (if (Utilities|DoesObjectImplementInterface OtherActor "/Game/Systems/Interaction/BPI_Interactable.BPI_Interactable_C")
    (Utilities|Array|AddUnique (Variables|Ref|GetInteractablesInRange) OtherActor)))

(event Custom|InteractBegin
  (bind _activeinteractable (CallFunction|GetActiveInteractable))
  (Utilities|IsValid _activeinteractable
    (:Is%20Valid
      (bind _type (Class|BPIInteractable|GetInteractionType(Message) _activeinteractable))
      (switch Utilities|FlowControl|Switch|SwitchonE_InteractionType _type ; Check the type selected on object
        (:NewEnumerator0
          (CallFunction|InteractwithActive) ; Interact instantly if the Type is "Press"
        )
        (:NewEnumerator1
          ;[0.15 0.15 0.15 0.5] When enum type is "Hold", bind an event and check if the elapsed time since pressed is greater than the wanted value
          (EventDispatchers|BindEventtoOnGoingInteractStart (delegate Custom|OnInteractionOnGoing)))))))

(event Custom|HandleRangeEndOverlap
  (params (OverlappedComponent :type Primitive%20Component%20Object%20Reference) (OtherActor :type Actor%20Object%20Reference) (OtherComp :type Primitive%20Component%20Object%20Reference) (OtherBodyIndex :type Integer))
  (bind _interactablesinrange (Variables|Ref|GetInteractablesInRange))
  ;[0.15 0.15 0.15 0.5] Remove the interactable actor when no more in range
  (if (Utilities|Array|ContainsItem _interactablesinrange OtherActor)
    (Utilities|Array|RemoveItem _interactablesinrange OtherActor)))

(event Custom|OnInteractionOnGoing
  (params (ElapsedSeconds :type Float%20%28double-precision%29))
  ;[0.15 0.15 0.15 0.5] When enum type is "Hold", bind an event and check if the elapsed time since pressed is greater than the wanted value
  (Development|PrintString (Utilities|String|ToString(Float) ElapsedSeconds) true true "(R=1.000000,G=0.000000,B=0.962142,A=1.000000)" 1.0 "ElapsedTimer")
  (if (> ElapsedSeconds 1.0)
    (CallFunction|InteractwithActive)
    (EventDispatchers|UnbindEventfromOnGoingInteractStart (delegate Custom|OnInteractionOnGoing))))

(event Custom|InteractWithActive
  ;[0.15 0.15 0.15 0.5] Final interaction logic (called only when pressed or hold completed
  (Class|BPIInteractable|Interact(Message) (CallFunction|GetActiveInteractable) (Variables|Ref|GetCharacterRef)))

(event Input|EnhancedActionEvents|EnhancedInputActionIA_Interact
  (params (ActionValue :type Boolean) (ElapsedSeconds :type Float%20%28double-precision%29) (TriggeredSeconds :type Float%20%28double-precision%29) (InputAction :type Input%20Action%20Object%20Reference :default "/Game/Input/Actions/IA_Interact.IA_Interact"))
  ;[0.15 0.15 0.15 0.5] Interaction input Handler
  (:Started
    (CallFunction|InteractBegin) ; Press event call
  )
  (:Ongoing
    (Default|CallOnGoingInteractStart ElapsedSeconds) ; Hold event dipatcher to avoid conflict
  )
  (:Canceled
    (EventDispatchers|UnbindallEventsfromOnGoingInteractStart :!label _label) ; Unbind all the events when the hold is completed or canceled
  )
  (:Completed
    (goto _label)))

(event EventBeginPlay
  (bind _ascharacter (Utilities|Casting|CastToCharacter (Components|GetOwner)))
  (Utilities|IsValid _ascharacter
    (:Is%20Valid
      (bind _output_get (Variables|Ref|SetCharacterRef _ascharacter))
      (bind _returnvalue (Game|AddComponentbyClass _output_get "/Script/Engine.SphereComponent" false))
      (bind _output_get_2 (Variables|Overlaps|SetRangeSphere _returnvalue))
      (Components|Sphere|SetSphereRadius _output_get_2 (Variables|Overlaps|GetRangeSphereRadius) true)
      (Development|SetHiddeninGame _output_get_2 (Variables|Overlaps|GetNewHidden) false)
      (Collision|BindEventtoOnComponentBeginOverlap (Variables|Overlaps|GetRangeSphere) (EventDispatchers|CreateEvent :!event Custom|HandleRangeBeginOverlap))
      (Collision|BindEventtoOnComponentEndOverlap (Variables|Overlaps|GetRangeSphere) (EventDispatchers|CreateEvent :!event Custom|HandleRangeEndOverlap)))))

(fn GetActiveInteractable
  (for (_array_element _array_index) (Variables|Ref|GetInteractablesInRange) ; Iterate over the actors in range
    (LocalVariables|SetCurrentActor _array_element)
    (if (== _array_index 0)
      ;[0.15 0.15 0.15 0.5] If it is the first actor in array set it to closest
      (LocalVariables|SetClosestActor (LocalVariables|GetCurrentActor))
      (else
        ;[0.15 0.15 0.15 0.5] Else find the closest to Character
        (LocalVariables|SetClosestActor (CallFunction|GetClosestActor (LocalVariables|GetCurrentActor) (LocalVariables|GetClosestActor))))))
  (return (LocalVariables|GetClosestActor)) ; End of the loop
)

(fn DitanceBeetwenActors
  (params (First :type Actor%20Object%20Reference) (Second :type Actor%20Object%20Reference))
  (return (Math|Vector|Distance(Vector) (Transformation|GetActorLocation First) (Transformation|GetActorLocation Second))))

(fn GetClosestActor
  (params (Current :type Actor%20Object%20Reference) (Other :type Actor%20Object%20Reference))
  (bind _characterref (Variables|Ref|GetCharacterRef))
  (if (< (CallFunction|DitanceBeetwenActors Current _characterref) (CallFunction|DitanceBeetwenActors Other _characterref))
    (return Current) ; Return Current
    (else
      (return Other) ; Return Other
    )))